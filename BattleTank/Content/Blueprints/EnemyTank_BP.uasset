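; EnemyTank_BP is the enemy tank Blueprint, which wires up the tank's aiming, movement and health bar when play begins.
; BeginPlay passes the turret and barrel to the TankAiming component and the left and right tracks to TankMovement.
; It then casts the widget component's user widget to EnemiesHealthBar and assigns itself as that widget's Tank.
; The Blueprint graph contains no other active logic.
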(event EventBeginPlay
  (Class|TankAimingComponent|InitializeAimingSystem (Variables|Default|GetTankAiming) (Variables|Default|GetTankTurret) (Variables|Default|GetTankBarrel))
  (Class|TankMovementComponent|InitializeTracks (Variables|Default|GetTankMovement) (Variables|Default|GetTankLeftTrack) (Variables|Default|GetTankRightTrack))
  (bind _asenemies_health_bar (Utilities|Casting|CastToEnemiesHealthBar (UserInterface|GetUserWidgetObject (Variables|Default|GetEnimiesHealthBarWidget))))
  (Variables|/Game/Blueprints/UI/EnemiesHealthBar.EnemiesHealthBar_C|SetTank _asenemies_health_bar self))

(event Collision|EventActorBeginOverlap
  (params (OtherActor :type Actor%20Object%20Reference)))

(event EventTick
  (params (DeltaSeconds :type Float%20%28single-precision%29)))

(fn ConstructionScript)